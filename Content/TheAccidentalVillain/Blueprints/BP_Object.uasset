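; BP_Object is an interactable object that carries a dialogue component and shows an interact prompt.
; On BeginPlay it creates a dialogue widget for BPDialogue, sets BPDialogue as the ACInteractable's parent and creates the prompt widget.
; Box overlap adds the "Interact" prompt to the viewport and removes it on exit.
; The BeginDialogue call in this graph is disconnected and never runs.
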(event `self.ReceiveBeginPlay`
  (bind _bp_dialogue (`self.BP_Dialogue`))
  (bind _returnvalue (`|CreateWidget` "/Game/TheAccidentalVillain/Blueprints/Dialogue/WBP_DialogueUI.WBP_DialogueUI_C" null _bp_dialogue))
  (set `/Game/TheAccidentalVillain/Blueprints/Dialogue/AC_Dialogue.DialogueUI` _returnvalue _bp_dialogue)
  (set `/Game/TheAccidentalVillain/Blueprints/AC_Interactable.Parent` (`self.BP_Dialogue`) (`self.AC_Interactable`))
  (bind _returnvalue_2 (`|CreateWidget` "/Game/TheAccidentalVillain/UI/UI_Interact.UI_Interact_C"))
  (set `self.UI` _returnvalue_2))

(event `self.Box.OnComponentBeginOverlap`
  (params (OverlappedComponent :type "PrimitiveComponent Object Reference") (OtherActor :type "Actor Object Reference") (OtherComp :type "PrimitiveComponent Object Reference") (OtherBodyIndex :type Integer) (bFromSweep :type Boolean) (SweepResult :type "HitResult Structure (by ref)"))
  (bind _ui (`self.UI`))
  (set `TextBlock.Text` "Interact" (`/Game/TheAccidentalVillain/UI/UI_Interact.TextBlock_29` _ui))
  (`UserWidget.AddToViewport` _ui 0))

(event `self.Box.OnComponentEndOverlap`
  (params (OverlappedComponent :type "PrimitiveComponent Object Reference") (OtherActor :type "Actor Object Reference") (OtherComp :type "PrimitiveComponent Object Reference") (OtherBodyIndex :type Integer))
  (`Widget.RemoveFromParent` (`self.UI`)))

(fn `UserConstructionScript`)