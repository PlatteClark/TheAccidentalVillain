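; BP_Pig is an ambient pig character that wanders at random until it dies.
; It starts patrolling on BeginPlay, moving to a random reachable point nearby, then idling for a random delay whether the move succeeds or fails.
; Each cycle rolls a random idle animation index, and one variant briefly raises a GetUp flag before moving again.
; Die sets IsDead, which stops the next patrol from starting.
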(event `self.ReceiveBeginPlay`
  (`self.GetNewPatrolLocation`))

(event `GetNewPatrolLocation`
  (set `self.IdleAnim` (`KismetMathLibrary.RandomIntegerInRange` 1 4))
  (`|AIMoveTo` self (`NavigationSystemV1.K2_GetRandomReachablePointInRadius` (`self.K2_GetActorLocation`) 500.0 null null) null
    (:`OnSuccess`
      _)
    (:`OnFail`
      _))
  (`KismetSystemLibrary.Delay` (`KismetMathLibrary.RandomFloatInRange` 4.0 8.0))
  (if (== (`self.IdleAnim`) 4)
    (set `self.GetUp` true)
    (`KismetSystemLibrary.Delay` 2.0)
    (set `self.GetUp` false))
  (if (not (`self.IsDead`))
    (`self.GetNewPatrolLocation`)))

(fn `Die`
  (set `self.IsDead` true))

(fn `UserConstructionScript`)