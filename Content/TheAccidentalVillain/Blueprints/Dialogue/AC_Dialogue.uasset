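; Dialogue component that steps through an array of dialogue sequences and displays NPC text in a UI widget.
; BeginDialogue adds the widget and starts the first sequence if none is current; otherwise its bounds check, which appears inverted, ends dialogue or advances.
; GetCurrentDialogue writes the indexed NPC line to the widget.
; NextDialogueSequence advances the sequence, while NextDialogue uses one index for both sequence and line, neither refreshing the text.
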(fn `BeginDialogue`
  (bind _dialogues (`self.Dialogues`))
  (bind _returnvalue (+ (`KismetArrayLibrary.Array_Find` _dialogues (`self.CurrentDialogue`)) 1))
  (`UserWidget.AddToViewport` (`self.DialogueUI`) 0)
  (if (`KismetArrayLibrary.Array_IsEmpty` (`.Dialogue_3_CD0E263F485565AAC3076095B994029C` (break `/Game/TheAccidentalVillain/Blueprints/Dialogue/F_DialogueSequence` (`self.CurrentDialogue`))))
    (set `self.CurrentDialogue` (`|GetArrayItem` (`self.Dialogues`)))
    (set `self.CurrentDialogueIndex` 0)
    (`self.GetCurrentDialogue` :!label _label)
    (elif (< _returnvalue (`KismetArrayLibrary.Array_Length` _dialogues))
      (`self.EndDialogue`)
      (else
        (set `self.CurrentDialogue` (`|GetArrayItem` _dialogues _returnvalue))
        (set `self.CurrentDialogueIndex` 0)
        (goto _label)))))

(fn `EndDialogue`
  (`Widget.RemoveFromParent` (`self.DialogueUI`)))

(fn `GetCurrentDialogue`
  (set `TextBlock.Text` (`KismetTextLibrary.Conv_StringToText` (`.NpcText_2_666662CC48E2DE64FEBDF3868CC72A4D` (break `/Game/TheAccidentalVillain/Blueprints/Dialogue/F_DialogueOption` (`|GetArrayItem` (`.Dialogue_3_CD0E263F485565AAC3076095B994029C` (break `/Game/TheAccidentalVillain/Blueprints/Dialogue/F_DialogueSequence` (`self.CurrentDialogue`))) (`self.CurrentDialogueIndex`))))) (`/Game/TheAccidentalVillain/Blueprints/Dialogue/WBP_DialogueUI.DialogueText` (`self.DialogueUI`))))

(fn `NextDialogue`
  (params (NextIndex :type Integer))
  (bind _output_get (set `self.CurrentDialogueIndex` NextIndex))
  (set `self.CurrentDialogue` (`|GetArrayItem` (`self.Dialogues`) _output_get)))

(fn `NextDialogueSequence`
  (bind _dialogues (`self.Dialogues`))
  (bind _returnvalue (`KismetArrayLibrary.Array_Find` _dialogues (`self.CurrentDialogue`)))
  (if (!= _returnvalue (`KismetArrayLibrary.Array_Length` _dialogues))
    (set `self.CurrentDialogue` (`|GetArrayItem` _dialogues (+ _returnvalue 1)))
    (set `self.CurrentDialogueIndex` 0)))