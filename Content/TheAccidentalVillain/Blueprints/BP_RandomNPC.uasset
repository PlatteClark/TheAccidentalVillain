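; BP_RandomNPC is a wandering NPC that offers randomly chosen dialogue.
; A looping patrol moves it to random reachable points nearby, pausing for a random delay after each success or failure.
; A repeating timer re-rolls its BPDialogue conversation and resets the line index while the dialogue UI is hidden.
; While that UI is visible, new moves wait and Tick halts movement and turns the NPC toward the player.
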(event `self.ReceiveBeginPlay`
  (`parent.ReceiveBeginPlay`)
  (`KismetSystemLibrary.K2_SetTimerDelegate` (delegate `RandomDialouge`) 1.0 true)
  (`self.GetNewPatrolLocation`))

(event `RandomDialouge`
  (bind _bp_dialogue (`self.BP_Dialogue`))
  (if (not (`Widget.IsVisible` (`/Game/TheAccidentalVillain/Blueprints/Dialogue/AC_Dialogue.DialogueUI` _bp_dialogue)))
    (set `/Game/TheAccidentalVillain/Blueprints/Dialogue/AC_Dialogue.CurrentDialogue` (`KismetArrayLibrary.Array_Random` (`/Game/TheAccidentalVillain/Blueprints/Dialogue/AC_Dialogue.Dialogues` _bp_dialogue)) _bp_dialogue)
    (set `/Game/TheAccidentalVillain/Blueprints/Dialogue/AC_Dialogue.CurrentDialogueIndex` 0 _bp_dialogue)))

(event `GetNewPatrolLocation`
  (bind _returnvalue (`KismetMathLibrary.RandomFloatInRange` 2.0 5.0))
  (if (`Widget.IsVisible` (`/Game/TheAccidentalVillain/Blueprints/Dialogue/AC_Dialogue.DialogueUI` (`self.BP_Dialogue`)))
    (`KismetSystemLibrary.Delay` _returnvalue)
    (else
      (`|AIMoveTo` self (`NavigationSystemV1.K2_GetRandomReachablePointInRadius` (`self.K2_GetActorLocation`) 500.0 null null) null
        (:`OnSuccess`
          _)
        (:`OnFail`
          _))
      (`KismetSystemLibrary.Delay` _returnvalue)))
  (`self.GetNewPatrolLocation`))

(event `self.ReceiveTick`
  (params (DeltaSeconds :type "Float (single-precision)"))
  (if (`Widget.IsVisible` (`/Game/TheAccidentalVillain/Blueprints/Dialogue/AC_Dialogue.DialogueUI` (`self.BP_Dialogue`)))
    (`MovementComponent.StopMovementImmediately` (`self.CharacterMovement`))
    (`self.K2_SetActorRotation` (`KismetMathLibrary.FindLookAtRotation` (`self.K2_GetActorLocation`) (`self.K2_GetActorLocation` (`GameplayStatics.GetPlayerPawn` 0))))))

(fn `UserConstructionScript`
  (`parent.UserConstructionScript`))