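; BP_EventHandler is an actor exposing scripted world events for The Accidental Villain: releasing the witch, killing pigs and burning the farm.
; ReleaseWitch and BurnFarm each create and play a level sequence, for the witch blowing up a house and the farm fire.
; KillPigs sets a timer by function name that later calls Die on every pig in PigsToKill.
; The event graph holds no logic, so the functions rely on being called.
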(fn `BurnFarm`
  (bind _outactor (`LevelSequencePlayer.CreateLevelSequencePlayer` "/Game/TheAccidentalVillain/Sequences/LS_FarmFire.LS_FarmFire"))
  (`MovieSceneSequencePlayer.Play` (`LevelSequenceActor.SequencePlayer` _outactor)))

(fn `KillPigs`
  (`KismetSystemLibrary.K2_SetTimer` null "KillPigsForReal" (`self.PigKillTimer`)))

(fn `KillPigsForReal`
  (for _array_element (`self.PigsToKill`)
    (`/Game/TheAccidentalVillain/Blueprints/BP_Pig.Die` _array_element)))

(fn `ReleaseWitch`
  (bind _outactor (`LevelSequencePlayer.CreateLevelSequencePlayer` "/Game/TheAccidentalVillain/Sequences/LS_WitchBlowsUpHouse.LS_WitchBlowsUpHouse"))
  (`MovieSceneSequencePlayer.Play` (`LevelSequenceActor.SequencePlayer` _outactor)))

(fn `UserConstructionScript`)